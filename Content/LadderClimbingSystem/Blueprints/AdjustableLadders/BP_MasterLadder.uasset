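; BP_MasterLadder is a ladder Blueprint that procedurally builds an adjustable-height ladder for the climbing system.
; Construction Script and BeginPlay both run AdjustLadder, which moves LadderTopAdjuster to LadderLength and rebuilds the geometry.
; AdjustHeight clears and refills instanced meshes, stacking rungs at FootBarSpread intervals and both side rails at SideDistance intervals up to the top.
; SyncedFootBar ties the rail cutoff to rung spacing instead of a fixed offset.
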(event Custom|AdjustLadder
  (bind _laddertopadjuster (Variables|Default|GetLadderTopAdjuster))
  (bind _relativelocation (Variables|/Script/Engine.SceneComponent|GetRelativeLocation _laddertopadjuster))
  ;[0.01562 0.01562 0.01562] Adjust Height
  ;;[0.02083 0.02083 0.02083] Set the length of the Ladder
  (Transformation|SetRelativeLocation _laddertopadjuster (Math|Vector|MakeVector (.x _relativelocation) (.y _relativelocation) (Variables|LadderSettings|GetLadderLength)) false false)
  (CallFunction|AdjustHeight))

(event EventBeginPlay
  ;[0.01042 0.01042 0.01042] Begin Play
  (CallFunction|AdjustLadder))

(fn ConstructionScript
  (CallFunction|AdjustLadder))

(fn AdjustHeight
  (bind _laddertopadjuster (Variables|Default|GetLadderTopAdjuster))
  (bind _relativelocation (Variables|/Script/Engine.SceneComponent|GetRelativeLocation _laddertopadjuster))
  ;[0.02083 0.02083 0.02083] Adjust Ladder Height
  ;;[0.01562 0.01562 0.01562 1 15] Reset Temp(Local) Height variable when adjusting the ladder (-20 to take into account for default Ladder length)
  (LocalVariables|SetLocalSideHeightStored -23.5)
  (LocalVariables|SetLocalBarHeightStored 0.0)
  ;;[0.02083 0.02083 0.02083 1 15] Check if Temp Height is Less than Bar Distance
  (Components|InstancedStaticMesh|ClearInstances (Variables|Default|GetLadderBarInstance))
  (while (< (LocalVariables|GetLocalBarHeightStored) (.Z (Math|Vector|BreakVector (Variables|/Script/Engine.SceneComponent|GetRelativeLocation (Variables|Default|GetLadderTopAdjuster)))))
    ;;[0.03125 0.03125 0.03125 1 15] Add a Mesh at the Temp Height Z Axis location (Will set at every interval of Distance)
    (Components|InstancedStaticMesh|AddInstance (Variables|Default|GetLadderBarInstance) (Math|Transform|MakeTransform (Math|Vector|MakeVector 0.0 0.0 (LocalVariables|GetLocalBarHeightStored)) "0, 0, 0" "1.000000,1.000000,1.000000") false)
    ;;[0.02604 0.02604 0.02604 1 15] Set Temp Height to the Current Temp Height + the Bar Distance
    (LocalVariables|SetLocalBarHeightStored (+ (LocalVariables|GetLocalBarHeightStored) (Variables|LadderSettings|GetFootBarSpread)))
    ;;[0.02083 0.02083 0.02083 1 15] Check if Temp Height is Less than Bar Distance
    (while (< (LocalVariables|GetLocalSideHeightStored) (.Z (Math|Vector|BreakVector (select (Variables|LadderSettings|GetbSyncedFootBar) (+ _relativelocation (* (Variables|LadderSettings|GetFootBarSpread) -1.0)) (+ _relativelocation -15.0)))))
      ;;[0.01562 0.01562 0.01562] Spawn Side Bar meshes
      (Components|InstancedStaticMesh|AddInstance (Variables|Default|GetLadderMidL) (Math|Transform|MakeTransform (Math|Vector|MakeVector 0.0 0.0 (LocalVariables|GetLocalSideHeightStored)) "0, 0, 0" "1.000000,1.000000,1.000000") false)
      (Components|InstancedStaticMesh|AddInstance (Variables|Default|GetLadderMidR) (Math|Transform|MakeTransform (Math|Vector|MakeVector 0.0 0.0 (LocalVariables|GetLocalSideHeightStored)) "0, 0, 0" "1.000000,1.000000,1.000000") false)
      ;;[0.01042 0.01042 0.01042] Set Value for Local Side Height Stored
      (LocalVariables|SetLocalSideHeightStored (+ (LocalVariables|GetLocalSideHeightStored) (Variables|DoNotEdit|GetSideDistance))))))