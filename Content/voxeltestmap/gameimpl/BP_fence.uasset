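; BP_fence marks a planned dig area with a closed spline-mesh fence, traced to the ground at the preview actor's corners, and runs digging there.
; While the player overlaps its box, it takes left-mouse input; holding plays dig montages and Tick fills a progress widget.
; On completion it adds a voxel stamp, spawns BP_holeID, adds dug volume to BP_game and briefly enables physics on "isexcavated" items inside.
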(event OnComponentBeginOverlap(Boxcollision)
  (params (OverlappedComponent :type Primitive%20Component%20Object%20Reference) (OtherActor :type Actor%20Object%20Reference) (OtherComp :type Primitive%20Component%20Object%20Reference) (OtherBodyIndex :type Integer) (bFromSweep :type Boolean) (SweepResult :type Hit%20Result%20Structure%20%28by%20ref%29))
  (bind _asbp_mythirdperson (Utilities|Casting|CastToBP_Mythirdperson OtherActor))
  (Variables|Default|SetBP_mythirdperson _asbp_mythirdperson)
  (Variables|Default|Setisinoverlap true)
  (Utilities|IsValid (Variables|Default|GetBP_mythirdperson)
    (:Is%20Valid
      (Variables|/Game/ThirdPerson/Blueprints/BP_Mythirdperson.BP_Mythirdperson_C|Setoverlapactor (Variables|Default|GetBP_mythirdperson) self)
      (Input|EnableInput (Game|GetPlayerController 0))
      (bind _output_get (Variables|/Game/ThirdPerson/Blueprints/BP_Mythirdperson.BP_Mythirdperson_C|Setisleftmouseenable (Variables|Default|GetBP_mythirdperson) false))
      (Development|PrintString (Utilities|String|Append "isleft: " (Utilities|String|ToString(Boolean) _output_get))))))

(event OnComponentEndOverlap(Boxcollision)
  (params (OverlappedComponent :type Primitive%20Component%20Object%20Reference) (OtherActor :type Actor%20Object%20Reference) (OtherComp :type Primitive%20Component%20Object%20Reference) (OtherBodyIndex :type Integer))
  (bind _bp_mythirdperson (Variables|Default|GetBP_mythirdperson))
  (Utilities|Casting|CastToBP_Mythirdperson OtherActor)
  (Variables|Default|Setisinoverlap false)
  (Utilities|IsValid _bp_mythirdperson
    (:Is%20Valid
      (Variables|/Game/ThirdPerson/Blueprints/BP_Mythirdperson.BP_Mythirdperson_C|Setoverlapactor _bp_mythirdperson 0)
      (Input|DisableInput (Game|GetPlayerController 0))
      (bind _output_get (Variables|/Game/ThirdPerson/Blueprints/BP_Mythirdperson.BP_Mythirdperson_C|Setisleftmouseenable (Variables|Default|GetBP_mythirdperson) true))
      (Development|PrintString (Utilities|String|Append "isleft: " (Utilities|String|ToString(Boolean) _output_get))))))

(event Custom|digvoxel
  (bind _bp_game (Variables|Default|GetBP_game))
  (bind _previewscale (Variables|Default|Getpreviewscale))
  (bind _bp_mythirdperson (Variables|Default|GetBP_mythirdperson))
  (bind _bp_mythirdperson_2 (Variables|Default|GetBP_mythirdperson))
  (bind _bp_mythirdperson_3 (Variables|Default|GetBP_mythirdperson))
  (bind (_x _y _z) (Math|Vector|BreakVector _previewscale))
  (bind _wbp_previewvolume (Variables|/Game/ThirdPerson/Blueprints/BP_Mythirdperson.BP_Mythirdperson_C|GetWBP_previewvolume _bp_mythirdperson))
  (bind _digpreviewref (Variables|/Game/ThirdPerson/Blueprints/BP_Mythirdperson.BP_Mythirdperson_C|GetDigpreviewref _bp_mythirdperson_2))
  (bind _returnvalue (Transformation|GetActorLocation _digpreviewref))
  (bind _returnvalue_2 (+ _z 1.0))
  (bind _returnvalue_3 (Math|Vector|MakeVector _x _y _returnvalue_2))
  (bind _returnvalue_4 (+ (.z _returnvalue) 1e+02))
  (Variables|/Game/ThirdPerson/Blueprints/BP_Mythirdperson.BP_Mythirdperson_C|Setbeforediglocation _bp_mythirdperson_3 (Transformation|GetActorLocation _bp_mythirdperson_3))
  (bind _copy (Class|VoxelStampK2|MakeCopy (Variables|/Game/ThirdPerson/Blueprints/BP_Mythirdperson.BP_Mythirdperson_C|GetNew%20Stamp (Variables|Default|GetBP_mythirdperson))))
  (bind _outstamp (Class|VoxelStampK2|SetTransform _copy (Math|Transform|MakeTransform (Math|Vector|MakeVector (.x _returnvalue) (.y _returnvalue) _returnvalue_4) "0, 0, 0" _returnvalue_3)))
  (Game|SpawnActorfromClass "/Game/voxeltestmap/gameimpl/BP_holeID.BP_holeID_C" (Math|Transform|MakeTransform (Math|Vector|MakeVector (.x _returnvalue) (.y _returnvalue) _returnvalue_4) "0, 0, 0" _returnvalue_3) "Undefined" "MultiplyWithRoot" 0 0)
  (Class|VoxelInstancedStampComponent|AddStamp (Variables|/Game/ThirdPerson/Blueprints/BP_Mythirdperson.BP_Mythirdperson_C|GetVoxelInstancedStamp (Variables|Default|GetBP_mythirdperson)) _outstamp)
  (Variables|/Game/voxeltestmap/gameimpl/BP_game.BP_game_C|Setvolume _bp_game (+ (Variables|/Game/voxeltestmap/gameimpl/BP_game.BP_game_C|Getvolume _bp_game) (/ (* (* (Variables|/Game/voxeltestmap/gameimpl/WBP_previewvolume.WBP_previewvolume_C|GetLength _wbp_previewvolume) (Variables|/Game/voxeltestmap/gameimpl/WBP_previewvolume.WBP_previewvolume_C|GetWidth _wbp_previewvolume)) (Variables|/Game/voxeltestmap/gameimpl/WBP_previewvolume.WBP_previewvolume_C|GetHeight _wbp_previewvolume)) 1e+06))))

(event Custom|removeui
  ;[0.15 0.15 0.15 0.5] ui
  (Utilities|IsValid (Variables|Default|GetWBP_digui)
    (:Is%20Valid
      (Widget|RemovefromParent (Variables|Default|GetWBP_digui))
      (Variables|Default|SetWBP_digui 0)
      (Variables|Default|SetCurrentDigTime 0.0))))

(event EventBeginPlay
  (bind _previewactor (Variables|Default|Getpreviewactor))
  (bind _boxcollision (Variables|Default|GetBoxcollision))
  (bind _boxcollison (Variables|/Game/voxeltestmap/gameimpl/BP_VoxelDigPreview.BP_VoxelDigPreview_C|Getboxcollison _previewactor))
  (bind _returnvalue (Transformation|GetWorldTransform _boxcollison))
  (Transformation|SetWorldRotation _boxcollision "0, 0, 0" false false)
  (Transformation|SetWorldScale3D _boxcollision (Math|Vector|MakeVector (.x (.scale _returnvalue)) (.y (.scale _returnvalue)) (+ (.z (.scale _returnvalue)) 3e+01)))
  (Variables|Default|Setpreviewscale (Variables|/Game/voxeltestmap/gameimpl/BP_VoxelDigPreview.BP_VoxelDigPreview_C|GetCurrentScale _previewactor))
  (bind _returnvalue_2 (Actor|GetActorOfClass "/Game/voxeltestmap/gameimpl/BP_game.BP_game_C"))
  (Variables|Default|SetBP_game _returnvalue_2))

(event Collision|EventActorBeginOverlap
  (params (OtherActor :type Actor%20Object%20Reference)))

(event EventTick
  (params (DeltaSeconds :type Float%20%28single-precision%29))
  (bind _wbp_digui (Variables|Default|GetWBP_digui))
  (if (Variables|Default|Getispressed)
    (if (Variables|Default|Getisinoverlap)
      ;[0.15 0.15 0.15 0.5] 挖掘进度条
      (bind _output_get (Variables|Default|SetCurrentDigTime (+ (Utilities|Time|GetWorldDeltaSeconds) (Variables|Default|GetCurrentDigTime))))
      (bind _output_get_2 (Variables|Default|Setpercent (/ _output_get (Variables|Default|Getdigduration))))
      (Utilities|IsValid _wbp_digui
        (:Is%20Valid
          (Progress|SetPercent (Variables|/Game/voxeltestmap/gameimpl/WBP_DigProgress.WBP_DigProgress_C|GetProgressBar _wbp_digui) _output_get_2)
          (if (>= (Variables|Default|GetCurrentDigTime) (Variables|Default|Getdigduration))
            (CallFunction|Digvoxel)
            (Utilities|FlowControl|Delay 0.2)
            (Variables|Default|Setisreadyfordig false)
            (Input|EnableInput (Variables|Default|GetBP_mythirdperson) (Game|GetPlayerController 0))
            (Variables|Default|Setisdigging false)
            (Default|StopMontageAllSk (Variables|Default|GetBP_mythirdperson))
            (CallFunction|Removeui)
            (Actor|DestroyActor (Variables|/Game/ThirdPerson/Blueprints/BP_Mythirdperson.BP_Mythirdperson_C|GetDigpreviewref (Variables|Default|GetBP_mythirdperson)))
            ;[0.15 0.15 0.15 0.5] 玩家视野中的物体实现物理模拟
            (bind _outactors (Collision|BoxOverlapActors (Variables|Default|Getpreori) (Variables|Default|Getpreext) (Utilities|Array|MakeArray "ObjectTypeQuery2" "ObjectTypeQuery1") "/Game/voxeltestmap/gameimpl/Observe/BP_ItemBase.BP_ItemBase_C" :!class /Script/Engine.KismetSystemLibrary))
            (for _array_element _outactors
              (if (Actor|ActorHasTag _array_element "isexcavated")
                (bind _asbp_item_base (Utilities|Casting|CastToBP_ItemBase _array_element))
                (Physics|SetSimulatePhysics (Variables|/Game/voxeltestmap/gameimpl/Observe/BP_ItemBase.BP_ItemBase_C|GetStaticMesh _asbp_item_base) true)
                (Utilities|FlowControl|Delay 2.0)
                (Physics|SetSimulatePhysics (Variables|/Game/voxeltestmap/gameimpl/Observe/BP_ItemBase.BP_ItemBase_C|GetStaticMesh _asbp_item_base) false)))))))))

(event Input|MouseEvents|LeftMouseButton
  (params (Key :type Key%20Structure :default "None"))
  (bind _bp_mythirdperson (Variables|Default|GetBP_mythirdperson))
  (:Pressed
    (Development|PrintString "fence")
    (Variables|Default|Setispressed true)
    (if (Variables|Default|Getisreadyfordig)
      (Variables|Default|Setisdigging true)
      (if (Variables|Default|Getisinoverlap)
        (Input|DisableInput (Variables|Default|GetBP_mythirdperson) (Game|GetPlayerController 0))
        (Animation|Montage|PlayMontage (Variables|/Game/ThirdPerson/Blueprints/BP_Mythirdperson.BP_Mythirdperson_C|GetSK_Chest _bp_mythirdperson) "/Game/voxeltestmap/AM_dig.AM_dig"
          (:then
            (Animation|Montage|PlayMontage (Variables|/Game/ThirdPerson/Blueprints/BP_Mythirdperson.BP_Mythirdperson_C|GetSK_Eyeglasses _bp_mythirdperson) "/Game/voxeltestmap/AM_dig.AM_dig"
              (:then
                (Animation|Montage|PlayMontage (Variables|/Game/ThirdPerson/Blueprints/BP_Mythirdperson.BP_Mythirdperson_C|GetSK_Hand/Glove _bp_mythirdperson) "/Game/voxeltestmap/AM_dig.AM_dig"
                  (:then
                    (Animation|Montage|PlayMontage (Variables|/Game/ThirdPerson/Blueprints/BP_Mythirdperson.BP_Mythirdperson_C|GetSK_Hair _bp_mythirdperson) "/Game/voxeltestmap/AM_dig.AM_dig"
                      (:then
                        (Animation|Montage|PlayMontage (Variables|/Game/ThirdPerson/Blueprints/BP_Mythirdperson.BP_Mythirdperson_C|GetSK_Hat _bp_mythirdperson) "/Game/voxeltestmap/AM_dig.AM_dig"
                          (:then
                            (Animation|Montage|PlayMontage (Variables|/Game/ThirdPerson/Blueprints/BP_Mythirdperson.BP_Mythirdperson_C|GetSK_Head _bp_mythirdperson) "/Game/voxeltestmap/AM_dig.AM_dig"
                              (:then
                                ;[0.15 0.15 0.15 0.5] ui
                                (Utilities|IsValid (Variables|Default|GetWBP_digui)
                                  (:Is%20Valid
                                    _)
                                  (:Is%20Not%20Valid
                                    (bind _returnvalue (UserInterface|CreateWidget "/Game/voxeltestmap/gameimpl/WBP_DigProgress.WBP_DigProgress_C" 0 self))
                                    (bind _output_get (Variables|Default|SetWBP_digui _returnvalue))))
                                (UserInterface|Viewport|AddtoViewport _output_get 0)
                                (Variables|Default|Setpreviewscale (Variables|/Game/voxeltestmap/gameimpl/BP_VoxelDigPreview.BP_VoxelDigPreview_C|GetCurrentScale (Variables|/Game/ThirdPerson/Blueprints/BP_Mythirdperson.BP_Mythirdperson_C|GetDigpreviewref (Variables|Default|GetBP_mythirdperson)))))))))))))))))))
  (:Released
    (Variables|Default|Setispressed false)
    (Variables|Default|Setisdigging false)
    (if (Variables|Default|Getisinoverlap)
      (Default|StopMontageAllSk _bp_mythirdperson))))

(fn ConstructionScript
  (bind _spline (Variables|Default|GetSpline))
  (bind _previewactor (Variables|Default|Getpreviewactor))
  (bind _spline_2 (Variables|Default|GetSpline))
  (bind _spline_3 (Variables|Default|GetSpline))
  (bind _previewactor_2 (Variables|Default|Getpreviewactor))
  (bind _previewactor_3 (Variables|Default|Getpreviewactor))
  (bind _previewactor_4 (Variables|Default|Getpreviewactor))
  (bind _returnvalue (Spline|GetNumberOfSplinePoints _spline))
  (bind (_origin _boxextent) (Collision|GetActorBounds _previewactor_2 false false))
  (bind (_origin_2 _boxextent_2) (Collision|GetActorBounds _previewactor_3 false false))
  (bind (_origin_3 _boxextent_3) (Collision|GetActorBounds _previewactor_4 false false))
  (bind (_origin_4 _boxextent_4) (Collision|GetActorBounds _previewactor false false))
  (bind (_origin_5 _boxextent_5) (Collision|GetActorBounds _previewactor_4 false false))
  (bind _returnvalue_2 (+ (.y _origin_3) (.y _boxextent_3)))
  (bind _returnvalue_3 (- (.x _origin) (.x _boxextent)))
  (bind _returnvalue_4 (- (.y _origin_4) (.y _boxextent_4)))
  (bind _returnvalue_5 (- (.x _origin_4) (.x _boxextent_4)))
  (bind _returnvalue_6 (+ (.y _origin) (.y _boxextent)))
  (bind _returnvalue_7 (+ (.x _origin_2) (.x _boxextent_2)))
  (bind _returnvalue_8 (- (.y _origin_2) (.y _boxextent_2)))
  (bind _returnvalue_9 (+ (.x _origin_3) (.x _boxextent_3)))
  (Utilities|FlowControl|Sequence
    (:then_0
      (Spline|ClearSplinePoints (Variables|Default|GetSpline) true)
      (Variables|Default|Setpreori _origin_5)
      (Variables|Default|Setpreext _boxextent_5)
      (bind _outhit (Collision|LineTraceByChannel (Math|Vector|MakeVector _returnvalue_9 _returnvalue_2 (+ (.z _origin_3) 1e+03)) (Math|Vector|MakeVector _returnvalue_9 _returnvalue_2 (- (.z _origin_3) 1e+03)) "TraceTypeQuery1" false 0 "Persistent"))
      (bind _output_get (Variables|Default|Setpoint0 (.Location (Collision|BreakHitResult _outhit))))
      (Spline|AddSplinePointatIndex (Variables|Default|GetSpline) _output_get 0 "World" true)
      (bind _outhit_2 (Collision|LineTraceByChannel (Math|Vector|MakeVector _returnvalue_7 _returnvalue_8 (+ (.z _origin_2) 1e+03)) (Math|Vector|MakeVector _returnvalue_7 _returnvalue_8 (- (.z _origin_2) 1e+03)) "TraceTypeQuery1" false 0 "Persistent"))
      (bind _output_get_2 (Variables|Default|Setpoint1 (.Location (Collision|BreakHitResult _outhit_2))))
      (Spline|AddSplinePointatIndex (Variables|Default|GetSpline) _output_get_2 1 "World" true)
      (bind _outhit_3 (Collision|LineTraceByChannel (Math|Vector|MakeVector _returnvalue_5 _returnvalue_4 (+ (.z _origin_4) 1e+03)) (Math|Vector|MakeVector _returnvalue_5 _returnvalue_4 (- (.z _origin_4) 1e+03)) "TraceTypeQuery1" false 0 "Persistent"))
      (bind _output_get_3 (Variables|Default|Setpoint2 (.Location (Collision|BreakHitResult _outhit_3))))
      (Spline|AddSplinePointatIndex (Variables|Default|GetSpline) _output_get_3 2 "World" true)
      (bind _outhit_4 (Collision|LineTraceByChannel (Math|Vector|MakeVector _returnvalue_3 _returnvalue_6 (+ (.z _origin) 1e+03)) (Math|Vector|MakeVector _returnvalue_3 _returnvalue_6 (- (.z _origin) 1e+03)) "TraceTypeQuery1" false 0 "Persistent"))
      (bind _output_get_4 (Variables|Default|Setpoint3 (.Location (Collision|BreakHitResult _outhit_4))))
      (Spline|AddSplinePointatIndex _spline_2 _output_get_4 3 "World" true)
      (Spline|SetClosedLoop _spline_2 true true))
    (:then_2
      (for _index (range 0 (- _returnvalue 1))
        (Development|PrintString "1111")
        (Spline|SetSplinePointType _spline _index "Linear" true)
        (bind _returnvalue_10 (AddComponent|AddSplineMeshComponent false))
        (Transformation|AttachComponentToComponent _returnvalue_10 (Variables|Default|GetDefaultSceneRoot) "None" "KeepRelative" "KeepRelative" "KeepRelative" true)
        (SplineMesh|SetStartandEnd _returnvalue_10 (.Location (Spline|GetLocationandTangentatSplinePoint _spline_3 _index "Local")) "0, 0, 0" (.Location (Spline|GetLocationandTangentatSplinePoint _spline_3 (Math|Integer|%(Integer) (+ _index 1) _returnvalue) "Local")) "0, 0, 0" true :!class /Script/Engine.SplineMeshComponent)))))