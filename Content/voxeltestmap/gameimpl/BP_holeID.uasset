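; BP_holeID marks a hole within a trench and gives it a sequential ID.
; On BeginPlay it increments the hole counter in BP_game and adds a record of ID, location, XY-scale area and trench ID to MapSystem's Holes array.
; When a BP_ItemBase overlaps its box, it writes the hole ID into the item's context field, but only if that field is not -1.
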(event OnComponentBeginOverlap(BoxCollision)
  (params (OverlappedComponent :type Primitive%20Component%20Object%20Reference) (OtherActor :type Actor%20Object%20Reference) (OtherComp :type Primitive%20Component%20Object%20Reference) (OtherBodyIndex :type Integer) (bFromSweep :type Boolean) (SweepResult :type Hit%20Result%20Structure%20%28by%20ref%29))
  (bind _asbp_item_base (Utilities|Casting|CastToBP_ItemBase OtherActor))
  (if (not (== (.context (Variables|/Game/voxeltestmap/gameimpl/Observe/BP_ItemBase.BP_ItemBase_C|Getitemstruct _asbp_item_base)) -1))
    (Variables|/Game/voxeltestmap/gameimpl/Observe/BP_ItemBase.BP_ItemBase_C|Setitemstruct _asbp_item_base (Utilities|Struct|MakeS_itemstruct (.name (Variables|/Game/voxeltestmap/gameimpl/Observe/BP_ItemBase.BP_ItemBase_C|Getitemstruct _asbp_item_base)) (.isstatckable (Variables|/Game/voxeltestmap/gameimpl/Observe/BP_ItemBase.BP_ItemBase_C|Getitemstruct _asbp_item_base)) (.image (Variables|/Game/voxeltestmap/gameimpl/Observe/BP_ItemBase.BP_ItemBase_C|Getitemstruct _asbp_item_base)) (.maxstatckablesize (Variables|/Game/voxeltestmap/gameimpl/Observe/BP_ItemBase.BP_ItemBase_C|Getitemstruct _asbp_item_base)) (.isconsumeable (Variables|/Game/voxeltestmap/gameimpl/Observe/BP_ItemBase.BP_ItemBase_C|Getitemstruct _asbp_item_base)) (.increasedata (Variables|/Game/voxeltestmap/gameimpl/Observe/BP_ItemBase.BP_ItemBase_C|Getitemstruct _asbp_item_base)) (.description (Variables|/Game/voxeltestmap/gameimpl/Observe/BP_ItemBase.BP_ItemBase_C|Getitemstruct _asbp_item_base)) (.class (Variables|/Game/voxeltestmap/gameimpl/Observe/BP_ItemBase.BP_ItemBase_C|Getitemstruct _asbp_item_base)) (.itemmesh (Variables|/Game/voxeltestmap/gameimpl/Observe/BP_ItemBase.BP_ItemBase_C|Getitemstruct _asbp_item_base)) (.isinlab (Variables|/Game/voxeltestmap/gameimpl/Observe/BP_ItemBase.BP_ItemBase_C|Getitemstruct _asbp_item_base)) (.labname (Variables|/Game/voxeltestmap/gameimpl/Observe/BP_ItemBase.BP_ItemBase_C|Getitemstruct _asbp_item_base)) (.labdescription (Variables|/Game/voxeltestmap/gameimpl/Observe/BP_ItemBase.BP_ItemBase_C|Getitemstruct _asbp_item_base)) (.note (Variables|/Game/voxeltestmap/gameimpl/Observe/BP_ItemBase.BP_ItemBase_C|Getitemstruct _asbp_item_base)) (.picturepath (Variables|/Game/voxeltestmap/gameimpl/Observe/BP_ItemBase.BP_ItemBase_C|Getitemstruct _asbp_item_base)) (.id (Variables|/Game/voxeltestmap/gameimpl/Observe/BP_ItemBase.BP_ItemBase_C|Getitemstruct _asbp_item_base)) (.type (Variables|/Game/voxeltestmap/gameimpl/Observe/BP_ItemBase.BP_ItemBase_C|Getitemstruct _asbp_item_base)) (.meterial (Variables|/Game/voxeltestmap/gameimpl/Observe/BP_ItemBase.BP_ItemBase_C|Getitemstruct _asbp_item_base)) (.dimension (Variables|/Game/voxeltestmap/gameimpl/Observe/BP_ItemBase.BP_ItemBase_C|Getitemstruct _asbp_item_base)) (.period (Variables|/Game/voxeltestmap/gameimpl/Observe/BP_ItemBase.BP_ItemBase_C|Getitemstruct _asbp_item_base)) (.conjecture (Variables|/Game/voxeltestmap/gameimpl/Observe/BP_ItemBase.BP_ItemBase_C|Getitemstruct _asbp_item_base)) (Variables|Default|Getholeid) (.catogory (Variables|/Game/voxeltestmap/gameimpl/Observe/BP_ItemBase.BP_ItemBase_C|Getitemstruct _asbp_item_base)) (.location_x (Variables|/Game/voxeltestmap/gameimpl/Observe/BP_ItemBase.BP_ItemBase_C|Getitemstruct _asbp_item_base)) (.location_y (Variables|/Game/voxeltestmap/gameimpl/Observe/BP_ItemBase.BP_ItemBase_C|Getitemstruct _asbp_item_base)) (.location_z (Variables|/Game/voxeltestmap/gameimpl/Observe/BP_ItemBase.BP_ItemBase_C|Getitemstruct _asbp_item_base)) (.test1 (Variables|/Game/voxeltestmap/gameimpl/Observe/BP_ItemBase.BP_ItemBase_C|Getitemstruct _asbp_item_base))))))

(event EventBeginPlay
  (bind _returnvalue (Transformation|GetActorLocation))
  (bind _returnvalue_2 (Transformation|GetActorScale3D))
  (bind _returnvalue_3 (Actor|GetActorOfClass "/Game/voxeltestmap/gameimpl/BP_game.BP_game_C"))
  (bind _output_get (Variables|Default|Setholeid (+ (Variables|/Game/voxeltestmap/gameimpl/BP_game.BP_game_C|Getholenum _returnvalue_3) 1)))
  (bind _output_get_2 (Variables|/Game/voxeltestmap/gameimpl/BP_game.BP_game_C|Setholenum _returnvalue_3 _output_get))
  (bind _returnvalue_4 (Actor|GetActorOfClass "/Game/voxeltestmap/gameimpl/map/MapSystem.MapSystem_C"))
  (bind _output_get_3 (Variables|Default|SetS%20Hole (Utilities|Struct|MakeS_hole _output_get_2 (.x _returnvalue) (.y _returnvalue) (.z _returnvalue) (* (.x _returnvalue_2) (.y _returnvalue_2)) (Variables|Default|Gettrenchid))))
  (Utilities|Array|Add (Variables|/Game/voxeltestmap/gameimpl/map/MapSystem.MapSystem_C|Getholes _returnvalue_4) _output_get_3))

(event Collision|EventActorBeginOverlap
  (params (OtherActor :type Actor%20Object%20Reference)))

(event EventTick
  (params (DeltaSeconds :type Float%20%28single-precision%29)))

(fn ConstructionScript)