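; BP_VoxelDigPreview is a preview actor for voxel digging, showing a resizable volume through its static mesh.
; BeginPlay caches the BP_Mythirdperson character and stores a dynamic MI_digpreview material instance on the mesh.
; UpdateBoxScale adds an offset to the stored scale, clamps the vector's length rather than each axis, applies it and prints it.
; An unconnected fragment would stop the player's movement and set IsInPre, but never runs.
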(event Custom|UpdateBoxScale
  (params (Offset :type Vector))
  (bind _output_get (Variables|Default|SetCurrentScale (Math|Vector|ClampVectorSize (+ Offset (Variables|Default|GetCurrentScale)) 1.0 1e+01)))
  (Transformation|SetActorScale3D _output_get)
  (Development|PrintString (Utilities|String|ToString(Vector) _output_get)))

(event EventBeginPlay
  (bind _returnvalue (Actor|GetActorOfClass "/Game/ThirdPerson/Blueprints/BP_Mythirdperson.BP_Mythirdperson_C"))
  (Variables|Default|SetBP_mythirdeperson _returnvalue)
  (bind _returnvalue_2 (Rendering|Material|CreateDynamicMaterialInstance (Variables|Default|GetStaticMesh) 0 "/Game/voxeltestmap/gameimpl/MI_digpreview.MI_digpreview" "None" :!class /Script/Engine.PrimitiveComponent))
  (Variables|Default|SetMI_pre _returnvalue_2))

(event Collision|EventActorBeginOverlap
  (params (OtherActor :type Actor%20Object%20Reference)))

(event EventTick
  (params (DeltaSeconds :type Float%20%28single-precision%29)))

(fn ConstructionScript)