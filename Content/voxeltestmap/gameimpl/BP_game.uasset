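; BP_game is a game manager actor that tracks a power budget and ends the game when it runs out.
; Each tick it subtracts Volume, scaled Totaldistance and a per-pit cost from Power.
; At zero or below it sets Isgameover, freezes the player character and shows WBP_gameover once, with UI-only input.
; BeginPlay caches all BP_holeID actors, which Inwhichbrenchfun searches to return a hole's trench ID.
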(event EventBeginPlay
  (bind _outactors (Actor|GetAllActorsOfClass "/Game/voxeltestmap/gameimpl/BP_holeID.BP_holeID_C"))
  (Variables|Default|Setholes _outactors))

(event Collision|EventActorBeginOverlap
  (params (OtherActor :type Actor%20Object%20Reference)))

(event EventTick
  (params (DeltaSeconds :type Float%20%28single-precision%29))
  (bind _returnvalue (Game|GetPlayerCharacter 0))
  (bind _returnvalue_2 (Game|GetPlayerController 0))
  (bind _charactermovement (Variables|/Script/Engine.Character|GetCharacterMovement _returnvalue))
  (if (<= (- (- (- (Variables|Default|Getpower) (Variables|Default|Getvolume)) (/ (Variables|Default|Gettotaldistance) 1e+03)) (* (Variables|Default|Getnumber) 10)) 0.0)
    (Variables|Default|Setisgameover true)
    (Components|Movement|StopMovementImmediately _charactermovement)
    (Variables|/Script/Engine.CharacterMovementComponent|SetMaxWalkSpeed _charactermovement 0.0)
    (Pawn|Components|CharacterMovement|SetMovementMode _charactermovement "MOVE_None" 0)
    (Utilities|IsValid (Variables|Default|GetWBP_gameover)
      (:Is%20Not%20Valid
        (bind _returnvalue_3 (UserInterface|CreateWidget "/Game/voxeltestmap/gameimpl/map/WBP_gameover.WBP_gameover_C" (Game|GetPlayerController 0)))
        (bind _output_get (Variables|Default|SetWBP_gameover _returnvalue_3))
        (UserInterface|Viewport|AddtoViewport _returnvalue_3 0)
        (Variables|/Script/Engine.PlayerController|SetbShowMouseCursor _returnvalue_2 true)
        (Input|SetInputModeUIOnly _returnvalue_2 _output_get "DoNotLock" false)))))

(fn ConstructionScript)

(fn Inwhichbrenchfun
  (params (holeid :type Integer))
  (for _array_element (Variables|Default|Getholes)
    (if (== (.id (Variables|/Game/voxeltestmap/gameimpl/BP_holeID.BP_holeID_C|GetS%20Hole _array_element)) holeid)
      (return (.trenchid (Variables|/Game/voxeltestmap/gameimpl/BP_holeID.BP_holeID_C|GetS%20Hole _array_element))))))