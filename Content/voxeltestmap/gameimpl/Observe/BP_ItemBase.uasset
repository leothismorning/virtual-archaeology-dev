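; Base world item that the player can inspect or pick up, with an excavation tag option.
; Construction builds its item struct from exposed fields and georeferenced coordinates, then configures the mesh.
; Sphere overlap toggles the interaction prompt; in dig-physics mode, both follow the mesh and any overlap stops simulation.
; Inspection spawns a far-off BP_inspectitem; pickup fills a missing icon from a temporary file, adds to interactor and game-mode inventories, then destroys itself.
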(event OnComponentBeginOverlap(SphereCollision)
  (params (OverlappedComponent :type Primitive%20Component%20Object%20Reference) (OtherActor :type Actor%20Object%20Reference) (OtherComp :type Primitive%20Component%20Object%20Reference) (OtherBodyIndex :type Integer) (bFromSweep :type Boolean) (SweepResult :type Hit%20Result%20Structure%20%28by%20ref%29))
  (if (== OtherActor (Game|GetPlayerCharacter 0))
    (Rendering|SetVisibility (Variables|Default|Getinteraction) true false))
  (if (Variables|Default|Getisdigchangephy)
    (Physics|SetSimulatePhysics (Variables|Default|GetStaticMesh) false)))

(event OnComponentEndOverlap(SphereCollision)
  (params (OverlappedComponent :type Primitive%20Component%20Object%20Reference) (OtherActor :type Actor%20Object%20Reference) (OtherComp :type Primitive%20Component%20Object%20Reference) (OtherBodyIndex :type Integer))
  (if (== OtherActor (Game|GetPlayerCharacter 0))
    (Rendering|SetVisibility (Variables|Default|Getinteraction) false false)))

(event EventBeginPlay
  (Variables|Default|SetPlayerref (CallFunction|FlibGetplayer))
  (bind _returnvalue (Actor|GetActorOfClass "/Game/voxeltestmap/gameimpl/inventory/BP_inventorygamemode.BP_inventorygamemode_C"))
  (Variables|Default|SetBP_inventorygamemode _returnvalue)
  (bind _geographiccoordinates (Class|GeoReferencingSystem|EnginetoGeographic (Class|GeoReferencingSystem|GetGeoReferencingSystem) (Transformation|GetActorLocation)))
  (Development|PrintString (Utilities|String|ToString(Float) (.latitude _geographiccoordinates)))
  (Development|PrintString (Utilities|String|ToString(Float) (.longitude _geographiccoordinates))))

(event Collision|EventActorBeginOverlap
  (params (OtherActor :type Actor%20Object%20Reference)))

(event EventTick
  (params (DeltaSeconds :type Float%20%28single-precision%29))
  (if (Variables|Default|Getisdigchangephy)
    (Transformation|SetWorldLocation (Variables|Default|GetSphereCollision) (+ (Transformation|GetWorldLocation (Variables|Default|GetStaticMesh)) "0.000000,0.000000,76.000000") false false)))

(event EventOninteract
  (params (character :type BP%20Mythirdperson%20Object%20Reference))
  (bind _itemscaleall (Variables|item|Getitemscaleall))
  (bind _itemstruct (Variables|Default|Getitemstruct))
  ;[0.15 0.15 0.15 0.5] 观看
  (bind _returnvalue (Game|SpawnActorfromClass "/Game/voxeltestmap/gameimpl/Observe/BP_inspectitem.BP_inspectitem_C" (Math|Transform|MakeTransform "100000000.000000,0.000000,0.000000") "Undefined" "MultiplyWithRoot" 0 self 0))
  (Default|Setinspectrotation _returnvalue (Variables|inspect|Getiteminspectrotation))
  (Default|Setinspectscale _returnvalue (Math|Vector|MakeVector _itemscaleall _itemscaleall _itemscaleall))
  (Class|BPIObserve|Inspect(Message) _returnvalue character (.itemmesh _itemstruct) (.name _itemstruct) (.description _itemstruct) (Variables|Default|Getisinworld) (Variables|Default|Getitemstruct)))

(event EventInterface
  (params (interactive :type Actor%20Object%20Reference))
  ;[0.15 0.15 0.15 0.5] 捡起来
  (Utilities|IsValid (.image (Utilities|Struct|BreakS_itemstruct (Variables|Default|Getitemstruct)))
    (:Is%20Valid
      _)
    (:Is%20Not%20Valid
      ;[0.15 0.15 0.15 0.5] 暂时的图片
      (bind _returnvalue (Class|KismetRenderingLibrary|ImportFileasTexture2D "Temp/MyPhoto.png"))
      (bind _output_get (Variables|Default|Setitemstruct (Utilities|Struct|MakeS_itemstruct (.name (Utilities|Struct|BreakS_itemstruct (Variables|Default|Getitemstruct))) (.isstatckable (Utilities|Struct|BreakS_itemstruct (Variables|Default|Getitemstruct))) _returnvalue (.maxstatckablesize (Utilities|Struct|BreakS_itemstruct (Variables|Default|Getitemstruct))) (.isconsumeable (Utilities|Struct|BreakS_itemstruct (Variables|Default|Getitemstruct))) (.increasedata (Utilities|Struct|BreakS_itemstruct (Variables|Default|Getitemstruct))) (.description (Utilities|Struct|BreakS_itemstruct (Variables|Default|Getitemstruct))) (.class (Utilities|Struct|BreakS_itemstruct (Variables|Default|Getitemstruct))) (.itemmesh (Utilities|Struct|BreakS_itemstruct (Variables|Default|Getitemstruct))) (.isinlab (Utilities|Struct|BreakS_itemstruct (Variables|Default|Getitemstruct))) (.labname (Utilities|Struct|BreakS_itemstruct (Variables|Default|Getitemstruct))) (.labdescription (Utilities|Struct|BreakS_itemstruct (Variables|Default|Getitemstruct))) (.note (Utilities|Struct|BreakS_itemstruct (Variables|Default|Getitemstruct))) (.picturepath (Utilities|Struct|BreakS_itemstruct (Variables|Default|Getitemstruct))) (.id (Utilities|Struct|BreakS_itemstruct (Variables|Default|Getitemstruct))) (.type (Utilities|Struct|BreakS_itemstruct (Variables|Default|Getitemstruct))) (.meterial (Utilities|Struct|BreakS_itemstruct (Variables|Default|Getitemstruct))) (.dimension (Utilities|Struct|BreakS_itemstruct (Variables|Default|Getitemstruct))) (.period (Utilities|Struct|BreakS_itemstruct (Variables|Default|Getitemstruct))) (.conjecture (Utilities|Struct|BreakS_itemstruct (Variables|Default|Getitemstruct))) (.context (Utilities|Struct|BreakS_itemstruct (Variables|Default|Getitemstruct))) (.catogory (Utilities|Struct|BreakS_itemstruct (Variables|Default|Getitemstruct))) (.location_x (Utilities|Struct|BreakS_itemstruct (Variables|Default|Getitemstruct))) (.location_y (Utilities|Struct|BreakS_itemstruct (Variables|Default|Getitemstruct))) (.location_z (Utilities|Struct|BreakS_itemstruct (Variables|Default|Getitemstruct))) (.test1 (Utilities|Struct|BreakS_itemstruct (Variables|Default|Getitemstruct))))))))
  (Default|Addslottoinventory (Actor|GetComponentbyClass interactive "/Game/voxeltestmap/gameimpl/inventory/BPC_inventory.BPC_inventory_C") (Utilities|Struct|MakeS_slotstruct _output_get 1))
  (Default|Addslottoinventory (Variables|/Game/voxeltestmap/gameimpl/inventory/BP_inventorygamemode.BP_inventorygamemode_C|GetBPC_inventory (Variables|Default|GetBP_inventorygamemode)) (Utilities|Struct|MakeS_slotstruct _output_get 1))
  (Actor|DestroyActor))

(fn ConstructionScript
  (bind _itemscaleall (Variables|item|Getitemscaleall))
  (bind _geographiccoordinates (Class|GeoReferencingSystem|EnginetoGeographic (Class|GeoReferencingSystem|GetGeoReferencingSystem) (Transformation|GetActorLocation)))
  (Variables|Default|Setitemstruct (Utilities|Struct|MakeS_itemstruct (Variables|item|Getitemname) false (Variables|Item|Getitemimage) 1 false 0.0 (Variables|item|Getitemdescription) 0 (Variables|item|Getitemmesh) false "" (Variables|item|Getdexcriptioninlab) "" "" 0 (Variables|item|Gettype) (Variables|item|Getmaterial) 0.0 "" "" (Variables|item|Getcontext) (Variables|item|Getcatogory) (.longitude _geographiccoordinates) (.latitude _geographiccoordinates) (.altitude _geographiccoordinates) (Variables|item|Getitemscaleall)))
  (Components|StaticMesh|SetStaticMesh (Variables|Default|GetStaticMesh) (Variables|item|Getitemmesh))
  (Transformation|SetWorldScale3D (Variables|Default|GetStaticMesh) (Math|Vector|MakeVector _itemscaleall _itemscaleall _itemscaleall))
  (if (Variables|item|Getisexcavated)
    (Variables|Default|SetTags (Utilities|Array|MakeArray "isexcavated"))))