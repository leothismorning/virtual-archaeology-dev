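; Item inspection actor that shows an item's mesh with a WBP_inspect widget, taking input from the player character until closed.
; Mouse input rotates or resets the mesh and zooms by changing the scene capture's clamped FOV.
; For items lacking an image, it exports RT_ldr after a short delay as a temp photo and a per-name PNG in Saved/itempictures, if absent.
; Closing restores input, removes the widget and destroys the actor.
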(event Custom|setinspectrotation
  (params (rotation :type Rotator))
  (bind _item (Variables|Default|Getitem))
  (bind _returnvalue (Transformation|GetWorldTransform _item))
  (bind _output_get (Variables|Default|SetiniRotation rotation))
  (Transformation|SetWorldTransform _item (Math|Transform|MakeTransform (.location _returnvalue) _output_get (.scale _returnvalue)) false false))

(event Custom|setinspectscale
  (params (scale :type Vector))
  (bind _item (Variables|Default|Getitem))
  (bind _returnvalue (Transformation|GetWorldTransform _item))
  (bind _output_get (Variables|Default|SetScale scale))
  (Transformation|SetWorldTransform _item (Math|Transform|MakeTransform (.location _returnvalue) (.rotation _returnvalue) _output_get) false false))

(event Custom|close
  (bind _returnvalue (Game|GetPlayerController 0))
  (bind _character (Variables|Default|GetCharacter))
  (bind _overlapactor (Variables|/Game/ThirdPerson/Blueprints/BP_Mythirdperson.BP_Mythirdperson_C|Getoverlapactor _character))
  (Input|DisableInput _returnvalue)
  (Input|EnableInput _character _returnvalue)
  (Utilities|IsValid _overlapactor
    (:Is%20Valid
      (Input|EnableInput _overlapactor _returnvalue))
    (:Is%20Not%20Valid
      _))
  (Utilities|IsValid (Variables|Default|GetinspectUI)
    (:Is%20Valid
      (Widget|RemovefromParent (Variables|Default|GetinspectUI))
      (Variables|Default|SetinspectUI 0)
      (Actor|DestroyActor))))

(event EventBeginPlay
  (Actor|GetActorOfClass "/Game/voxeltestmap/gameimpl/inventory/BP_inventorygamemode.BP_inventorygamemode_C"))

(event Collision|EventActorBeginOverlap
  (params (OtherActor :type Actor%20Object%20Reference)))

(event EventTick
  (params (DeltaSeconds :type Float%20%28single-precision%29)))

(event EventInspect
  (params (character :type BP%20Mythirdperson%20Object%20Reference) (inspectitem :type Static%20Mesh%20Object%20Reference) (itemname :type Text) (itemdescription :type Text) (isinworld :type Boolean) (itemstruct :type S%20Itemstruct%20Structure))
  (bind _returnvalue (Utilities|String|ToString(Text) itemname))
  (bind _returnvalue_2 (Game|GetPlayerController 0))
  (bind _returnvalue_3 (Class|KismetSystemLibrary|GetProjectSavedDirectory))
  (bind _scenecapturecomponent2dldr (Variables|Default|GetSceneCaptureComponent2Dldr))
  (bind _returnvalue_4 (Utilities|String|Append _returnvalue "_" "picture.png"))
  (bind _returnvalue_5 (Utilities|String|Append _returnvalue_3 "itempictures/"))
  (Variables|Default|SetCharacter character)
  (Components|StaticMesh|SetStaticMesh (Variables|Default|Getitem) inspectitem)
  (bind _returnvalue_6 (UserInterface|CreateWidget "/Game/voxeltestmap/gameimpl/Observe/WBP_inspect.WBP_inspect_C" 0 itemname itemdescription inspectitem isinworld (Variables|Default|Getinspectactor)))
  (bind _output_get (Variables|Default|SetinspectUI _returnvalue_6))
  (UserInterface|Viewport|AddtoViewport _output_get 0)
  (Input|DisableInput (Variables|Default|GetCharacter) _returnvalue_2)
  (Utilities|IsValid (Variables|/Game/ThirdPerson/Blueprints/BP_Mythirdperson.BP_Mythirdperson_C|Getoverlapactor (Variables|Default|GetCharacter))
    (:Is%20Valid
      (Input|DisableInput (Variables|/Game/ThirdPerson/Blueprints/BP_Mythirdperson.BP_Mythirdperson_C|Getoverlapactor (Variables|Default|GetCharacter)) 0))
    (:Is%20Not%20Valid
      _))
  (Input|EnableInput _returnvalue_2)
  (Utilities|FlowControl|Delay 0.5)
  (Utilities|IsValid (.image (Utilities|Struct|BreakS_itemstruct itemstruct))
    (:Is%20Not%20Valid
      ;[0.15 0.15 0.15 0.5] 将观看到的第一帧记录为图片
      (Rendering|ExportRenderTarget "/Game/voxeltestmap/gameimpl/Observe/RT_ldr.RT_ldr" "Temp/" "MyPhoto.png")
      ;[0.15 0.15 0.15 0.5] 保存到本地
      (if (not (Class|BlueprintPathsLibrary|FileExists (Utilities|String|Append _returnvalue_5 _returnvalue_4)))
        (Rendering|ExportRenderTarget "/Game/voxeltestmap/gameimpl/Observe/RT_ldr.RT_ldr" _returnvalue_5 _returnvalue_4)
        (Variables|/Script/Engine.SceneCaptureComponent|SetbCaptureEveryFrame _scenecapturecomponent2dldr false)
        (Variables|/Script/Engine.SceneCaptureComponent|SetbCaptureOnMovement _scenecapturecomponent2dldr false)))))

(event Input|MouseEvents|MouseX
  (params (AxisValue :type Float%20%28single-precision%29))
  (bind _item (Variables|Default|Getitem))
  (if (Variables|Default|Getrotate?)
    (Transformation|SetWorldRotation _item (Math|Rotator|CombineRotators (Transformation|GetWorldRotation _item) (Math|Rotator|MakeRotator 0.0 0.0 (* AxisValue -3.0))) false false)))

(event Input|MouseEvents|MouseY
  (params (AxisValue :type Float%20%28single-precision%29))
  (bind _item (Variables|Default|Getitem))
  (if (Variables|Default|Getrotate?)
    (Transformation|SetWorldRotation _item (Math|Rotator|CombineRotators (Transformation|GetWorldRotation _item) (Math|Rotator|MakeRotator 0.0 (* AxisValue -3.0) 0.0)) false false)))

(event Input|MouseEvents|LeftMouseButton
  (params (Key :type Key%20Structure))
  (:Pressed
    (Variables|Default|Setrotate? true))
  (:Released
    (Variables|Default|Setrotate? false)))

(event Input|MouseEvents|RightMouseButton
  (params (Key :type Key%20Structure))
  (:Pressed
    (Transformation|SetWorldRotation (Variables|Default|Getitem) (Variables|Default|GetiniRotation) false false)
    (Variables|/Script/Engine.SceneCaptureComponent2D|SetFOVAngle (Variables|Default|GetSceneCaptureComponent2D) 5e+01)))

(event Input|MouseEvents|MouseWheelUp
  (params (Key :type Key%20Structure))
  (bind _scenecapturecomponent2d (Variables|Default|GetSceneCaptureComponent2D))
  (:Pressed
    (Variables|/Script/Engine.SceneCaptureComponent2D|SetFOVAngle _scenecapturecomponent2d (Math|Float|Clamp(Float) (- (Variables|/Script/Engine.SceneCaptureComponent2D|GetFOVAngle _scenecapturecomponent2d) 2.0) 3e+01 8e+01))))

(event Input|MouseEvents|MouseWheelDown
  (params (Key :type Key%20Structure))
  (bind _scenecapturecomponent2d (Variables|Default|GetSceneCaptureComponent2D))
  (:Pressed
    (Variables|/Script/Engine.SceneCaptureComponent2D|SetFOVAngle _scenecapturecomponent2d (Math|Float|Clamp(Float) (+ (Variables|/Script/Engine.SceneCaptureComponent2D|GetFOVAngle _scenecapturecomponent2d) 2.0) 3e+01 8e+01))))

(fn ConstructionScript)